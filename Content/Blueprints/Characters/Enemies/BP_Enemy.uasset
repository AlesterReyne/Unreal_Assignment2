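; Enemy character that patrols between random BP_PatrolPoint actors, chases the player and triggers game over on reaching them.
; A Tick-driven state machine (Patrol, LookingPlayer, Attack, Waiting, Dead) sets speed, facing and movement input directly.
; Sight is a range check plus line trace after snapping toward the player, so detection is omnidirectional.
; Timers gate attack and cause tiredness until the next patrol point; TakeDamage handles death.
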(event `self.ReceiveBeginPlay`
  (set `self.CurrentHealth` (`self.MaxHealth`))
  (set `self.NotTired` true)
  (set `self.EnemyState` "NewEnumerator0")
  (`self.GetRandomPatrolPoint`))

(event `self.ReceiveTick`
  (params (DeltaSeconds :type "Float (single-precision)"))
  (bind _returnvalue (`GameplayStatics.GetPlayerPawn` 0))
  (bind _currentpatrolpoint (`self.CurrentPatrolPoint`))
  (bind _charactermovement (`self.CharacterMovement`))
  (set `self.CurrentFrameTimeDelta` DeltaSeconds)
  (if (not (`|EnumEquality` (`self.EnemyState`) "NewEnumerator4"))
    (bind _seeplayer (`self.CanSeePlayer`))
    (if (and _seeplayer (`self.NotTired`) (`|EnumInequality` (`self.EnemyState`) "NewEnumerator2"))
      (set `self.EnemyState` "NewEnumerator1"))
    (switch `/Game/Blueprints/Characters/Enemies/E_EnemyState` (`self.EnemyState`)
      (:`NewEnumerator0`
        (set `CharacterMovementComponent.MaxWalkSpeed` 100.0 _charactermovement)
        ; Patrol
        (set `self.AttackingPlayerTimer` 0.0)
        (set `self.FindingPlayerTimer` 0.0)
        (`self.RotateToTarget` _currentpatrolpoint)
        (`self.AddMovementInput` (`KismetMathLibrary.Normal` (- (`self.K2_GetActorLocation` _currentpatrolpoint) (`self.K2_GetActorLocation`))))
        (bind _isinrange (`self.isInRange` _currentpatrolpoint 200.0))
        (if _isinrange
          (set `self.NotTired` true)
          (`self.GetRandomPatrolPoint`)
          (set `self.EnemyState` "NewEnumerator3")))
      (:`NewEnumerator1`
        ; Looking for Player
        (set `CharacterMovementComponent.MaxWalkSpeed` 0.0 _charactermovement)
        (`self.RotateToTarget` _returnvalue)
        (bind _output_get (set `self.FindingPlayerTimer` (+ (`self.CurrentFrameTimeDelta`) (`self.FindingPlayerTimer`))))
        (if (>= _output_get (`self.TimeToLookPlayer`))
          (bind _seeplayer_2 (`self.CanSeePlayer`))
          (if _seeplayer_2
            (set `self.EnemyState` "NewEnumerator2")
            (else
              (set `self.EnemyState` "NewEnumerator0")))))
      (:`NewEnumerator2`
        (set `CharacterMovementComponent.MaxWalkSpeed` 1000.0 _charactermovement)
        ; Attack
        (bind _seeplayer_3 (`self.CanSeePlayer`))
        (if _seeplayer_3
          (`self.RotateToTarget` _returnvalue)
          (`self.AddMovementInput` (`KismetMathLibrary.Normal` (- (`self.K2_GetActorLocation` _returnvalue) (`self.K2_GetActorLocation`))) 0.5)
          (bind _isinrange_2 (`self.isInRange` _returnvalue 100.0))
          (if _isinrange_2
            (`self.OnGameOver`)
            (else
              (bind _output_get_2 (set `self.AttackingPlayerTimer` (+ (`self.AttackingPlayerTimer`) (`self.CurrentFrameTimeDelta`))))
              (if (>= _output_get_2 (`self.TimeToAttackPlayer`))
                (set `self.NotTired` false)
                (set `self.EnemyState` "NewEnumerator0"))))
          (else
            (set `self.FindingPlayerTimer` 0.0)
            (set `self.EnemyState` "NewEnumerator1"))))
      (:`NewEnumerator3`
        (set `CharacterMovementComponent.MaxWalkSpeed` 0.0 _charactermovement)
        (`KismetSystemLibrary.Delay` 2.0)
        (set `self.EnemyState` "NewEnumerator0"))
      (:`NewEnumerator4`
        (if true
          _)))))

(fn `CanSeePlayer`
  (returns (SeePlayer :type Boolean))
  (bind _returnvalue (`GameplayStatics.GetPlayerPawn` 0))
  (bind _returnvalue_2 (`self.K2_GetActorLocation`))
  (bind _isinrange (`self.isInRange` _returnvalue 1000.0))
  (if _isinrange
    (`self.RotateToTarget` _returnvalue)
    (bind _outhit (`KismetSystemLibrary.LineTraceSingleByProfile` :`Start` _returnvalue_2 :`End` (+ _returnvalue_2 (* (`self.GetActorForwardVector`) 10000.0)) :`ProfileName` "Pawn" :`DrawDebugType` "ForDuration")))
  (return (and _isinrange (== (`.HitActor` (`GameplayStatics.BreakHitResult` _outhit)) _returnvalue))))

(fn `GetRandomPatrolPoint`
  (bind _outactors (`GameplayStatics.GetAllActorsOfClass` "/Game/Blueprints/Characters/Enemies/BP_PatrolPoint.BP_PatrolPoint_C"))
  (set `self.CurrentPatrolPoint` (`|GetArrayItem` _outactors (`KismetMathLibrary.RandomIntegerInRange` 0 (- (`KismetArrayLibrary.Array_Length` _outactors) 1)))))

(fn `isInRange`
  (params (Object :type "Actor Object Reference") (Range :type "Float (double-precision)"))
  (returns (isInRange :type Boolean))
  (return (<= (`self.GetDistanceTo` Object) Range)))

(fn `RotateToTarget`
  (params (Target :type "Actor Object Reference"))
  (bind (_returnvalue_roll _returnvalue_pitch _returnvalue_yaw) (`KismetMathLibrary.BreakRotator` (`self.K2_GetActorRotation`)))
  (bind (_returnvalue_roll_2 _returnvalue_pitch_2 _returnvalue_yaw_2) (`KismetMathLibrary.BreakRotator` (`KismetMathLibrary.NormalizedDeltaRotator` (`KismetMathLibrary.FindLookAtRotation` (`self.K2_GetActorLocation`) (`self.K2_GetActorLocation` Target)) (`self.K2_GetActorRotation`))))
  (`self.K2_SetActorRotation` (`KismetMathLibrary.MakeRotator` 0.0 0.0 (+ _returnvalue_yaw_2 _returnvalue_yaw))))

(fn `TakeDamage`
  (params (Damage :type Integer))
  (if (not (`|EnumEquality` (`self.EnemyState`) "NewEnumerator4"))
    (bind _output_get (set `self.CurrentHealth` (- (`self.CurrentHealth`) Damage)))
    (if (<= _output_get 0)
      (set `self.EnemyState` "NewEnumerator4")
      (`self.OnDeath`)
      (else
        (`KismetSystemLibrary.PrintString` (`KismetStringLibrary.Concat_StrStr` "Enemy Health: " (`KismetStringLibrary.Conv_IntToString` _output_get)) true true (struct :`G` 0.66 :`B` 1.0 :`A` 1.0) 5.0)))))

(fn `UserConstructionScript`)