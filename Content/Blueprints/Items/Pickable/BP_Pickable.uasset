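; BP_Pickable is a pickup item that spins in the world and reacts when the player touches it.
; Each Tick increments SpeedRotation and applies it as the actor's yaw, so the spin rate depends on frame rate.
; Overlap with player 0's BP_Player pawn calls OnPickup, which only plays a 2D pickup sound and leaves the actor in place.
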(event `self.ReceiveTick`
  (params (DeltaSeconds :type "Float (single-precision)"))
  (bind _result (`/Engine/EditorBlueprintResources/StandardMacros.IncrementFloat` (`self.SpeedRotation`))
    (:`  `
      (`self.K2_SetActorRotation` (`KismetMathLibrary.MakeRotator` 0.0 0.0 _result)))))

(event `self.ReceiveActorBeginOverlap`
  (params (OtherActor :type "Actor Object Reference"))
  (cast `/Game/Blueprints/Characters/Player/BP_Player` OtherActor)
  (if (== OtherActor (`GameplayStatics.GetPlayerPawn` 0))
    (`self.OnPickup`)))

(fn `OnPickup`
  (`GameplayStatics.PlaySound2D` "/Game/Audio/SFX/SFX_Pickup.SFX_Pickup" 1.0 1.0 0.0 null null))

(fn `UserConstructionScript`)