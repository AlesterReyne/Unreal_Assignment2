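; BP_Pickable_Weapon is a child pickable item that grants the player a weapon when picked up.
; Its OnPickup override runs the parent logic, casts the player 0 pawn to BP_Player and activates the weapon matching its WeaponType.
; It then prints the type as a debug string and destroys itself; the event graph holds only disabled default nodes.
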(fn `OnPickup`
  (bind _weapontype (`self.WeaponType`))
  (`parent.OnPickup`)
  (bind _asbp_player (cast `/Game/Blueprints/Characters/Player/BP_Player` (`GameplayStatics.GetPlayerPawn` 0)))
  (`/Game/Blueprints/Characters/Player/BP_Player.ActivateWeapon` _asbp_player _weapontype)
  (`KismetSystemLibrary.PrintString` (`|GetEnumeratorNameAsString` _weapontype))
  (`self.K2_DestroyActor`))

(fn `UserConstructionScript`
  (`parent.UserConstructionScript`))