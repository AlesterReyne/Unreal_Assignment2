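; BP_Pickable_Magazine is an ammo pickup that reloads the player's active weapon of matching caliber.
; On BeginPlay it rolls a bullet count within a caliber-specific range, tints its visual and shows the count as text.
; OnPickup runs the parent logic, then scans the player's BP_WeaponBase components for an active weapon of the same type.
; A match passes the bullets to the player's ReloadWeapon and destroys the magazine.
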(event `self.ReceiveBeginPlay`
  (if (`|EnumEquality` (`self.Calliber`) "NewEnumerator0")
    (bind _output_get (set `self.Bullets` (`KismetMathLibrary.RandomIntegerInRange` 10 20)))
    (`PrimitiveComponent.SetMaterial` (`self.Visual`) 0 "/Game/Materials/Red.Red")
    (`TextRenderComponent.K2_SetText` (`self.Ammo`) (`KismetTextLibrary.Conv_IntToText` _output_get))
    (elif (`|EnumEquality` (`self.Calliber`) "NewEnumerator1")
      (bind _output_get_2 (set `self.Bullets` (`KismetMathLibrary.RandomIntegerInRange` 5 10)))
      (`PrimitiveComponent.SetMaterial` (`self.Visual`) 0 "/Game/Materials/White.White")
      (`TextRenderComponent.K2_SetText` (`self.Ammo`) (`KismetTextLibrary.Conv_IntToText` _output_get_2)))))

(fn `OnPickup`
  (`parent.OnPickup`)
  (bind _asbp_player (cast `/Game/Blueprints/Characters/Player/BP_Player` (`GameplayStatics.GetPlayerPawn` 0)))
  (for _array_element (`self.K2_GetComponentsByClass` _asbp_player "/Game/Blueprints/Items/Weapons/BP_WeaponBase.BP_WeaponBase_C")
    (if (and (`/Game/Blueprints/Items/Weapons/BP_WeaponBase.isWeaponActive` _array_element) (`|EnumEquality` (`self.Calliber`) (`/Game/Blueprints/Items/Weapons/BP_WeaponBase.WeaponType` _array_element)))
      (`/Game/Blueprints/Characters/Player/BP_Player.ReloadWeapon` _asbp_player _array_element (`self.Bullets`))
      (`self.K2_DestroyActor`))))

(fn `UserConstructionScript`
  (`parent.UserConstructionScript`))