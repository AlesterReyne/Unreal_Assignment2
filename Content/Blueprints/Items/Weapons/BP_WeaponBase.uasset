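; Base weapon component that handles shooting, ammo, reloading and active state for the player's weapons.
; On the shoot input, an active weapon with ammo spawns a physics-driven BP_Bullet at the player's barrel pivot, launches it with a forward impulse and destroys it after a short delay.
; SetWeaponActive toggles visibility and records possession, while Reload adds ammo capped at the maximum.
; Shooting and reloading broadcast ammo changes through an event dispatcher.
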(event `EnhancedInput|/Game/Input/IA_Shoot`
  (params (ActionValue :type Boolean) (ElapsedSeconds :type "Float (double-precision)") (TriggeredSeconds :type "Float (double-precision)") (InputAction :type "InputAction Object Reference" :default "/Game/Input/IA_Shoot.IA_Shoot"))
  (bind _currentammo (`self.CurrentAmmo`))
  (:`Triggered`
    (if (`self.isWeaponActive`)
      (if (> _currentammo 0)
        (`|ExecutionSequence`
          (:`then_0`
            (`/Engine/EditorBlueprintResources/StandardMacros.DecrementInt` _currentammo
              (:`  `
                (bind _asbp_player (cast `/Game/Blueprints/Characters/Player/BP_Player` (`GameplayStatics.GetPlayerPawn` 0)))
                (bind _returnvalue (`|SpawnActorFromClass` "/Game/Blueprints/Items/Weapons/BP_Bullet.BP_Bullet_C" (`KismetMathLibrary.MakeTransform` (`self.K2_GetComponentLocation` (`/Game/Blueprints/Characters/Player/BP_Player.Barrel Pivot` _asbp_player))) "Undefined" "MultiplyWithRoot" null (`self.Damage`) null))
                (bind _sphere (`/Game/Blueprints/Items/Weapons/BP_Bullet.Sphere` _returnvalue))
                (`PrimitiveComponent.SetSimulatePhysics` _sphere true)
                (`PrimitiveComponent.AddImpulse` _sphere (* (`Actor.GetActorForwardVector` (`GameplayStatics.GetPlayerPawn` 0)) 10000.0) "None" false)
                (`GameplayStatics.PlaySound2D` "/Game/Audio/SFX/SFX_Rifle_Shoot.SFX_Rifle_Shoot" 1.0 1.0 0.0 null null false)
                (`self.OnBulletsAmountChange`)
                (`KismetSystemLibrary.Delay` 1.0)
                (`Actor.K2_DestroyActor` _returnvalue)))))
        (else
          (`GameplayStatics.PlaySound2D` "/Game/Audio/SFX/SFX_Empty_Chamber_.SFX_Empty_Chamber_" 1.0 1.0 0.0 null null))))))

(fn `Reload`
  (params (Ammo :type Integer))
  (bind _maxammo (`self.MaxAmmo`))
  (bind _returnvalue (+ Ammo (`self.CurrentAmmo`)))
  (`|ExecutionSequence`
    (:`then_0`
      (if (>= _returnvalue _maxammo)
        (set `self.CurrentAmmo` _maxammo)
        (else
          (set `self.CurrentAmmo` _returnvalue))))
    (:`then_1`
      (`self.OnBulletsAmountChange`))))

(fn `SetWeaponActive`
  (params (isActive :type Boolean))
  (`self.SetVisibility` isActive true)
  (set `self.isWeaponActive` isActive)
  (if isActive
    (set `self.isWeaponInPlayerPossesion` true)))