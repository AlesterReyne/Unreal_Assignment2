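; GM_Shooter is the shooter game mode that shows the HUD and detects when all enemies are dead.
; On BeginPlay it adds the UWG_HUD widget to the viewport, counts every BP_Enemy in the level and binds to each one's OnDeath event.
; Each death increments a kill counter, and when it matches the initial enemy count a VICTORY message is printed on screen.
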(event `self.ReceiveBeginPlay`
  (bind _returnvalue (`|CreateWidget` "/Game/Blueprints/UI/UWG_HUD.UWG_HUD_C"))
  (`UserWidget.AddToViewport` _returnvalue 0)
  (set `self.KilledEnemy` 0)
  (bind _outactors (`GameplayStatics.GetAllActorsOfClass` "/Game/Blueprints/Characters/Enemies/BP_Enemy.BP_Enemy_C"))
  (`|ExecutionSequence`
    (:`then_0`
      (set `self.EnemyAmount` (`KismetArrayLibrary.Array_Length` _outactors)))
    (:`then_1`
      (for _array_element _outactors
        (add `/Game/Blueprints/Characters/Enemies/BP_Enemy.OnDeath` _array_element (delegate `OnEnemyDeath_Event`))))))

(event `OnEnemyDeath_Event`
  (bind _output_get (set `self.KilledEnemy` (+ (`self.KilledEnemy`) 1)))
  (if (== (`self.EnemyAmount`) _output_get)
    (`KismetSystemLibrary.PrintString` "VICTORY" true true (struct :`R` 0.093431 :`G` 0.520833 :`B` 0.058274 :`A` 1.0) 180.0)))

(fn `UserConstructionScript`)