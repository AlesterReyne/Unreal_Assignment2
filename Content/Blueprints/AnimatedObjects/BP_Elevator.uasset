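; BP_Elevator is an animated actor that moves vertically from the position where it is placed.
; On BeginPlay it stores its start location and plays the UpAndDown timeline, with no trigger or player input.
; Each update sets the Z offset to Alpha times Speed times MaxHeight without sweeping, so Speed scales travel distance rather than playback rate.
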(event `self.ReceiveBeginPlay`
  (bind (_startposition_x _startposition_y _startposition_z) (`KismetMathLibrary.BreakVector` (`self.StartPosition`)))
  (set `self.StartPosition` (`self.K2_GetActorLocation`))
  (bind (_direction _alpha) (`Timeline|UpAndDown`)
    (:`Update`
      (`self.K2_SetActorLocation` (`KismetMathLibrary.MakeVector` _startposition_x _startposition_y (+ _startposition_z (* (* _alpha (`self.Speed`)) (`self.MaxHeight`))))))))

(fn `UserConstructionScript`)